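; Audio trigger volume that plays a sound at random intervals and positions while the player is inside it.
; The construction script sizes and enables overlaps on a selectable sphere, box or capsule; entering starts a self-restarting random timer and leaving clears it.
; Each sound spawns at a random local-axis offset from the player or the actor.
; Debug mode prints and spawns visualizers at separately rolled positions, not necessarily the sound's.
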(event `self.ReceiveBeginPlay`
  ;[1 1 1] Check for player and start
  (for _array_element (`self.GetOverlappingActors` null)
    (if (== (`GameplayStatics.GetPlayerCharacter` 0) _array_element)
      (`KismetSystemLibrary.K2_SetTimer` null "Sound_Trig" (`KismetMathLibrary.RandomFloatInRange` (`self.Time_Min`) (`self.TIme_Max`)) :!label _label))))

(event `Retrigger`
  ;[1 1 1] Check for player and start
  (goto _label))

(event `self.ReceiveActorBeginOverlap`
  (params (OtherActor :type "Actor Object Reference"))
  ;[1 1 1] Check for player and start
  (if (== (`GameplayStatics.GetPlayerCharacter` 0) OtherActor)
    (goto _label)))

(event `self.ReceiveActorEndOverlap`
  (params (OtherActor :type "Actor Object Reference"))
  ;[1 1 1] Check for player and start
  (if (== (`GameplayStatics.GetPlayerCharacter` 0) OtherActor)
    (`KismetSystemLibrary.K2_ClearTimer` null "Sound_Trig")))

(event `Sound_Trig`
  (bind _returnvalue (select `bool` (`self.Player_Origin`) :`false` self :`true` (`GameplayStatics.GetPlayerCharacter` 0) :!type "Actor Object Reference"))
  (bind _returnvalue_2 (+ (`self.K2_GetActorLocation` _returnvalue) (+ (* (`self.GetActorForwardVector` _returnvalue) (`KismetMathLibrary.RandomFloatInRange` (.x (`self.Min`)) (.x (`self.Max`)))) (* (`self.GetActorRightVector` _returnvalue) (`KismetMathLibrary.RandomFloatInRange` (.y (`self.Min`)) (.y (`self.Max`)))) (* (`self.GetActorUpVector` _returnvalue) (`KismetMathLibrary.RandomFloatInRange` (.z (`self.Min`)) (.z (`self.Max`)))))))
  ;[1 1 1] Spawn sound
  (`GameplayStatics.SpawnSoundAtLocation` (`self.Sound`) _returnvalue_2 (struct) (`self.Volume`) 1.0 0.0 null null)
  (`self.Retrigger`)
  (if (`self.Debug`)
    ;[1 1 1] Debug
    (`KismetSystemLibrary.PrintString` (`KismetStringLibrary.Conv_VectorToString` _returnvalue_2))
    (`|SpawnActorFromClass` "/Game/HorrorEngine/Blueprints/UsableAssets/Audio/Blueprints/POS_Test_Visualizer.POS_Test_Visualizer_C" (`KismetMathLibrary.Conv_VectorToTransform` _returnvalue_2) "Undefined" "OverrideRootScale" null null)))

(fn `UserConstructionScript`
  (bind _sphere (`self.Sphere`))
  (bind _box (`self.Box`))
  (bind _capsule (`self.Capsule`))
  (switch `/Game/HorrorEngine/Blueprints/UsableAssets/Audio/Blueprints/Audio_POS_Shape` (`self.Shape`)
    (:`NewEnumerator0`
      (`SphereComponent.SetSphereRadius` _sphere (`self.Sphere_Radius`) true)
      (set `PrimitiveComponent.bGenerateOverlapEvents` true _sphere))
    (:`NewEnumerator1`
      (`BoxComponent.SetBoxExtent` _box (`self.Box_Extents`) true)
      (set `PrimitiveComponent.bGenerateOverlapEvents` true _box))
    (:`NewEnumerator2`
      (`CapsuleComponent.SetCapsuleSize` _capsule (`self.Capsule_Radius`) (`self.Capsule_Half_Height`) true)
      (set `PrimitiveComponent.bGenerateOverlapEvents` true _capsule))))