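; Blueprint function library that gets and sets the PSX-style retro rendering effects.
; Most pairs read and write MPC_PSXFX parameters for dithering, color quantization, vertex snapping, affine mapping, depth error, polygon draw distance and near clip.
; Screen percentage and upscale smoothing instead go through console commands and console variables.
; Some setters clamp their inputs, and the affine toggle is stored as a float scalar.
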(fn `DisableUpscaleSmoothing`
  (params (Disabled :type Boolean :default false))
  (`KismetSystemLibrary.ExecuteConsoleCommand` null (`KismetStringLibrary.Concat_StrStr` "r.Upscale.Quality " (`KismetStringLibrary.Conv_IntToString` (`KismetMathLibrary.Conv_BoolToInt` (not Disabled)))) null)
  (return))

(fn `GetColorQuantization`
  (returns (R :type "Float (double-precision)") (G :type "Float (double-precision)") (B :type "Float (double-precision)"))
  (bind _returnvalue (`KismetMaterialLibrary.GetVectorParameterValue` null "/Game/PSXFX/Materials/MPC_PSXFX.MPC_PSXFX" "RGB Quantize"))
  (return (break `LinearColor` _returnvalue) (`.G` (break `LinearColor` _returnvalue)) (`.B` (break `LinearColor` _returnvalue))))

(fn `GetDepthError`
  (returns (Depth :type "Float (double-precision)") (Sensitivity :type "Float (double-precision)"))
  (bind _returnvalue (`KismetMaterialLibrary.GetScalarParameterValue` null "/Game/PSXFX/Materials/MPC_PSXFX.MPC_PSXFX" "Depth Error Sensitivity"))
  (bind _returnvalue_2 (`KismetMaterialLibrary.GetScalarParameterValue` null "/Game/PSXFX/Materials/MPC_PSXFX.MPC_PSXFX" "Depth Error"))
  (return _returnvalue_2 _returnvalue))

(fn `GetDitherIntensity`
  (returns (ReturnValue :type "Float (double-precision)"))
  (bind _returnvalue (`KismetMaterialLibrary.GetScalarParameterValue` null "/Game/PSXFX/Materials/MPC_PSXFX.MPC_PSXFX" "Dither Intensity"))
  (return _returnvalue))

(fn `GetDrawDistance`
  (returns (ReturnValue :type "Float (double-precision)"))
  (bind _returnvalue (`KismetMaterialLibrary.GetScalarParameterValue` null "/Game/PSXFX/Materials/MPC_PSXFX.MPC_PSXFX" "Polygon Draw Distance"))
  (return _returnvalue))

(fn `GetDrawDistanceGridSize`
  (returns (ReturnValue :type "Float (double-precision)"))
  (bind _returnvalue (`KismetMaterialLibrary.GetScalarParameterValue` null "/Game/PSXFX/Materials/MPC_PSXFX.MPC_PSXFX" "Draw Distance Grid Size"))
  (return _returnvalue))

(fn `GetNearClipDistance`
  (returns (ReturnValue :type "Float (double-precision)"))
  (bind _returnvalue (`KismetMaterialLibrary.GetScalarParameterValue` null "/Game/PSXFX/Materials/MPC_PSXFX.MPC_PSXFX" "Near Clip Distance"))
  (return _returnvalue))

(fn `GetScreenPercentage`
  (returns (ReturnValue :type "Float (double-precision)"))
  (bind _returnvalue (`KismetSystemLibrary.GetConsoleVariableFloatValue` "r.ScreenPercentage"))
  (return _returnvalue))

(fn `GetVertexSnap`
  (returns (GridSizeX :type Integer) (GridSizeY :type Integer))
  (bind _returnvalue (`KismetMaterialLibrary.GetScalarParameterValue` null "/Game/PSXFX/Materials/MPC_PSXFX.MPC_PSXFX" "Grid Size Y"))
  (bind _returnvalue_2 (`KismetMaterialLibrary.GetScalarParameterValue` null "/Game/PSXFX/Materials/MPC_PSXFX.MPC_PSXFX" "Grid Size X"))
  (return (`KismetMathLibrary.FTrunc` _returnvalue_2) (`KismetMathLibrary.FTrunc` _returnvalue)))

(fn `IsAffineMappingEnabled`
  (returns (ReturnValue :type Boolean))
  (bind _returnvalue (`KismetMaterialLibrary.GetScalarParameterValue` null "/Game/PSXFX/Materials/MPC_PSXFX.MPC_PSXFX" "Affine Toggle"))
  (return (`KismetMathLibrary.Conv_IntToBool` (`KismetMathLibrary.Round` _returnvalue))))

(fn `IsUpscaleSmoothingDisabled`
  (returns (ReturnValue :type Boolean))
  (bind _returnvalue (`KismetSystemLibrary.GetConsoleVariableIntValue` "r.Upscale.Quality"))
  (return (== _returnvalue 0)))

(fn `SetAffineMappingEnabled`
  (params (Enabled :type Boolean :default false))
  (`KismetMaterialLibrary.SetScalarParameterValue` null "/Game/PSXFX/Materials/MPC_PSXFX.MPC_PSXFX" "Affine Toggle" (`KismetMathLibrary.Conv_BoolToDouble` Enabled))
  (return))

(fn `SetColorQuantization`
  (params (R :type "Float (double-precision)" :default 128.0) (G :type "Float (double-precision)" :default 128.0) (B :type "Float (double-precision)" :default 128.0))
  (`KismetMaterialLibrary.SetVectorParameterValue` null "/Game/PSXFX/Materials/MPC_PSXFX.MPC_PSXFX" "RGB Quantize" (make `LinearColor` R G B))
  (return))

(fn `SetDepthError`
  (params (Depth :type "Float (double-precision)" :default 0.0) (Sensitivity :type "Float (double-precision)" :default 0.0))
  (`KismetMaterialLibrary.SetScalarParameterValue` null "/Game/PSXFX/Materials/MPC_PSXFX.MPC_PSXFX" "Depth Error" Depth)
  (`KismetMaterialLibrary.SetScalarParameterValue` null "/Game/PSXFX/Materials/MPC_PSXFX.MPC_PSXFX" "Depth Error Sensitivity" Sensitivity)
  (return))

(fn `SetDitherIntensity`
  (params (Intensity :type "Float (double-precision)" :default 0.0))
  (`KismetMaterialLibrary.SetScalarParameterValue` null "/Game/PSXFX/Materials/MPC_PSXFX.MPC_PSXFX" "Dither Intensity" (`KismetMathLibrary.FClamp` Intensity))
  (return))

(fn `SetDrawDistance`
  (params (Distance :type "Float (double-precision)"))
  (`KismetMaterialLibrary.SetScalarParameterValue` null "/Game/PSXFX/Materials/MPC_PSXFX.MPC_PSXFX" "Polygon Draw Distance" (`KismetMathLibrary.FMax` Distance))
  (return))

(fn `SetDrawDistanceGridSize`
  (params (Size :type "Float (double-precision)"))
  (`KismetMaterialLibrary.SetScalarParameterValue` null "/Game/PSXFX/Materials/MPC_PSXFX.MPC_PSXFX" "Draw Distance Grid Size" (`KismetMathLibrary.FMax` Size 1.0))
  (return))

(fn `SetNearClipDistance`
  (params (Distance :type "Float (double-precision)"))
  (`KismetMaterialLibrary.SetScalarParameterValue` null "/Game/PSXFX/Materials/MPC_PSXFX.MPC_PSXFX" "Near Clip Distance" (`KismetMathLibrary.FMax` Distance))
  (return))

(fn `SetScreenPercentage`
  (params (Percent :type "Float (double-precision)" :default 100.0))
  (`KismetSystemLibrary.ExecuteConsoleCommand` null (`KismetStringLibrary.Concat_StrStr` "r.ScreenPercentage " (`KismetStringLibrary.Conv_DoubleToString` (`KismetMathLibrary.FClamp` Percent 10.0 400.0))) null)
  (return))

(fn `SetVertexSnap`
  (params (GridSizeX :type Integer :default 5000) (GridSizeY :type Integer :default 5000))
  (`KismetMaterialLibrary.SetScalarParameterValue` null "/Game/PSXFX/Materials/MPC_PSXFX.MPC_PSXFX" "Grid Size X" (`KismetMathLibrary.Conv_IntToDouble` GridSizeX))
  (`KismetMaterialLibrary.SetScalarParameterValue` null "/Game/PSXFX/Materials/MPC_PSXFX.MPC_PSXFX" "Grid Size Y" (`KismetMathLibrary.Conv_IntToDouble` GridSizeY))
  (return))